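; BP_HJ_Enemy is an enemy Blueprint that shows a health bar when the player is nearby.
; Each tick it copies max and current HP from its Fsm into the HJ_UI_EnemyHP_Bar widget.
; Overlap of its Sphere with Player_KYI shows the bar, and ending the overlap hides it.
; Tick also hides the bar whenever current HP equals zero.
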(event `self.ReceiveTick`
  (params (DeltaSeconds :type "Float (single-precision)"))
  (`self.UpdateHealthBar`)
  (if (== (`EnemyFSM.currHP` (`self.fsm`)) 0.0)
    (`SceneComponent.SetVisibility` (`self.HealthBar`) false false)))

(event `self.ReceiveBeginPlay`)

(event `self.Sphere.OnComponentBeginOverlap`
  (params (OverlappedComponent :type "PrimitiveComponent Object Reference") (OtherActor :type "Actor Object Reference") (OtherComp :type "PrimitiveComponent Object Reference") (OtherBodyIndex :type Integer) (bFromSweep :type Boolean) (SweepResult :type "HitResult Structure (by ref)"))
  ;[1 1 1] HP Bar 보여주기
  (cast `Player_KYI` OtherActor)
  (`SceneComponent.SetVisibility` (`self.HealthBar`) true false))

(event `self.Sphere.OnComponentEndOverlap`
  (params (OverlappedComponent :type "PrimitiveComponent Object Reference") (OtherActor :type "Actor Object Reference") (OtherComp :type "PrimitiveComponent Object Reference") (OtherBodyIndex :type Integer))
  ;[1 1 1] HP Bar 보여주기
  (cast `Player_KYI` OtherActor)
  (`SceneComponent.SetVisibility` (`self.HealthBar`) false false))

(fn `UpdateHealthBar`
  (bind _fsm (`self.fsm`))
  (bind _ashj_ui_enemy_hp_bar (cast `/Game/HJ_other/UI/HJ_UI_EnemyHP_Bar` (`WidgetComponent.GetUserWidgetObject` (`self.HealthBar`))))
  (set `/Game/HJ_other/UI/HJ_UI_EnemyHP_Bar.maxHealth` (`EnemyFSM.maxHP` _fsm) _ashj_ui_enemy_hp_bar)
  (set `/Game/HJ_other/UI/HJ_UI_EnemyHP_Bar.Health` (`EnemyFSM.currHP` _fsm) _ashj_ui_enemy_hp_bar)
  (return))

(fn `UserConstructionScript`)