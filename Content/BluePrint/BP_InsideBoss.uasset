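; BP_InsideBoss is a trigger actor that opens the InsideBossUI screen when the player (Player_KYI) enters its Box.
; After a short delay, the begin overlap pauses the game, adds the widget to the viewport, switches input to UI-only and shows the mouse cursor.
; When the player leaves the Box, it hides the Inside component; nothing here unpauses the game or restores input.
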(event `self.Box.OnComponentBeginOverlap`
  (params (OverlappedComponent :type "PrimitiveComponent Object Reference") (OtherActor :type "Actor Object Reference") (OtherComp :type "PrimitiveComponent Object Reference") (OtherBodyIndex :type Integer) (bFromSweep :type Boolean) (SweepResult :type "HitResult Structure (by ref)"))
  (bind _returnvalue (`GameplayStatics.GetPlayerController` 0))
  (cast `Player_KYI` OtherActor)
  (`KismetSystemLibrary.Delay` 0.5)
  (`GameplayStatics.SetGamePaused` true)
  (bind _returnvalue_2 (`|CreateWidget` "/Game/HJ_other/UI/InsideBossUI.InsideBossUI_C"))
  (`UserWidget.AddToViewport` _returnvalue_2 0)
  (`WidgetBlueprintLibrary.SetInputMode_UIOnlyEx` _returnvalue null)
  (set `PlayerController.bShowMouseCursor` true _returnvalue))

(event `self.Box.OnComponentEndOverlap`
  (params (OverlappedComponent :type "PrimitiveComponent Object Reference") (OtherActor :type "Actor Object Reference") (OtherComp :type "PrimitiveComponent Object Reference") (OtherBodyIndex :type Integer))
  (cast `Player_KYI` OtherActor)
  (`SceneComponent.SetVisibility` (`self.Inside`) false false))

(fn `UserConstructionScript`)