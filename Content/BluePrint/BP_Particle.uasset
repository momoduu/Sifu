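; Particle trigger actor that sends the player to the BossUIMap level when they enter its box.
; The Wqwee component activates on BeginPlay and on player overlap, and deactivates when the Player_KYI leaves.
; Any overlap plays the Magic1 sound; for the player, a delay then shows the DarkUI widget and opens the level.
; Leaving the box does not cancel the pending transition.
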(event `self.ReceiveBeginPlay`
  (`ActorComponent.SetActive` (`self.wqwee`) true false))

(event `self.box.OnComponentBeginOverlap`
  (params (OverlappedComponent :type "PrimitiveComponent Object Reference") (OtherActor :type "Actor Object Reference") (OtherComp :type "PrimitiveComponent Object Reference") (OtherBodyIndex :type Integer) (bFromSweep :type Boolean) (SweepResult :type "HitResult Structure (by ref)"))
  (`GameplayStatics.PlaySound2D` "/Game/HJ_other/Sound/Magic1.Magic1" 2.0 1.0 0.0 null null)
  (cast `Player_KYI` OtherActor)
  (`ActorComponent.SetActive` (`self.wqwee`) true false)
  (`KismetSystemLibrary.Delay` 5.0)
  (bind _returnvalue (`|CreateWidget` "/Game/HJ_other/UI/DarkUI.DarkUI_C"))
  (`UserWidget.AddToViewport` _returnvalue 0)
  (`GameplayStatics.OpenLevel` "BossUIMap"))

(event `self.box.OnComponentEndOverlap`
  (params (OverlappedComponent :type "PrimitiveComponent Object Reference") (OtherActor :type "Actor Object Reference") (OtherComp :type "PrimitiveComponent Object Reference") (OtherBodyIndex :type Integer))
  (cast `Player_KYI` OtherActor)
  (`ActorComponent.SetActive` (`self.wqwee`) false false))

(fn `UserConstructionScript`)