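; BP_HJ_Boss is a boss Blueprint that keeps its health bar widget in sync with its health.
; Every Tick it calls UpdateHpbar, which casts Hpbar to FinalUI and copies max and current HP from the Bfsm component into it.
; Tick also checks for zero current HP, but that branch does nothing yet.
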(event `self.ReceiveTick`
  (params (DeltaSeconds :type "Float (single-precision)"))
  (`self.updateHpbar`)
  (if (== (`BossFSM.currHP` (`self.bfsm`)) 0.0)
    _))

(fn `updateHpbar`
  (bind _bfsm (`self.bfsm`))
  (bind _asfinal_ui (cast `/Game/HJ_other/UI/FinalUI` (`self.hpbar`)))
  (set `/Game/HJ_other/UI/FinalUI.maxHPbar` (`BossFSM.maxHP` _bfsm) _asfinal_ui)
  (set `/Game/HJ_other/UI/FinalUI.HPbar` (`BossFSM.currHP` _bfsm) _asfinal_ui)
  (return))

(fn `UserConstructionScript`)