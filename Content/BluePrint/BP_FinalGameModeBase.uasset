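; Game mode for the final boss fight that drives both HUDs and decides the win or lose ending.
; BeginPlay finds the HJ_Boss, casts the player pawn to Player_KYI and creates the player and boss UI widgets.
; Tick copies both HP values into the widgets and opens the winning or losing level after a delay, checking boss death first.
; The boss death sound has no once-only guard, so it fires every tick.
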(event `self.ReceiveBeginPlay`
  (bind _returnvalue (`GameplayStatics.GetActorOfClass` "/Script/Sifu.HJ_Boss"))
  (set `self.boss` _returnvalue)
  (bind _asplayer_kyi (cast `Player_KYI` (`GameplayStatics.GetPlayerPawn` 0)))
  (set `self.player` _asplayer_kyi)
  (bind _returnvalue_2 (`|CreateWidget` "/Game/SideScrollerBP/UI/PlayerUI.PlayerUI_C"))
  (bind _output_get (set `self.playerUI` _returnvalue_2))
  (`UserWidget.AddToViewport` _output_get 0)
  (bind _returnvalue_3 (`|CreateWidget` "/Game/HJ_other/UI/FinalUI.FinalUI_C"))
  (bind _output_get_2 (set `self.bossUI` _returnvalue_3))
  (`UserWidget.AddToViewport` _output_get_2 0))

(event `self.ReceiveTick`
  (params (DeltaSeconds :type "Float (single-precision)"))
  (bind _bossui (`self.bossUI`))
  (bind _playerui (`self.playerUI`))
  (bind _player (`self.player`))
  (bind _bfsm (`HJ_Boss.bfsm` (`self.Boss`)))
  (set `/Game/HJ_other/UI/FinalUI.HPbar` (`BossFSM.currHP` _bfsm) _bossui)
  (set `/Game/HJ_other/UI/FinalUI.maxHPbar` (`BossFSM.maxHP` _bfsm) _bossui)
  (set `/Game/SideScrollerBP/UI/PlayerUI.currentHP` (`Player_KYI.currHp` _player) _playerui)
  (set `/Game/SideScrollerBP/UI/PlayerUI.maxHP` (`Player_KYI.maxHp` _player) _playerui)
  (if (<= (`BossFSM.currHP` (`HJ_Boss.bfsm` (`self.Boss`))) 0.0)
    (`GameplayStatics.PlaySound2D` "/Game/HJ_other/Sound/Die2.Die2" 1.0 1.0 0.0 null null)
    (`KismetSystemLibrary.Delay` 3.0)
    (`GameplayStatics.OpenLevel` "WinningEnding")
    (elif (<= (`Player_KYI.currHp` (`self.player`)) 0.0)
      (`KismetSystemLibrary.Delay` 3.0)
      (`GameplayStatics.OpenLevel` "LosingEnding"))))

(fn `UserConstructionScript`)